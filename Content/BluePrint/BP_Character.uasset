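; BP_Character is the player character Blueprint, handling jump, movement, look, swimming, damage and death.
; Movement input follows control rotation, and movement mode changes set IsSwimming and the rotation rate, restoring a yaw-only actor rotation outside water.
; Damage is ignored while any montage plays; otherwise it lowers clamped Health and plays a hit montage.
; At zero Health it ragdolls the mesh, disables movement and calls game over once.
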(event `Key|SpaceBar`
  (params (Key :type "Key Structure"))
  ;[1 1 1 1 15] Character control
  (:`Pressed`
    (`self.Jump`)))

(event `InputAxis|MoveForward`
  (params (AxisValue :type "Float (single-precision)"))
  ;[1 1 1 1 15] Character control
  ;[1 1 1 1 15] Adding character control - Swimming
  (if (`self.Is Swimming?`)
    (`self.AddMovementInput` (`KismetMathLibrary.GetForwardVector` (`self.GetControlRotation`)) AxisValue)
    (else
      (`self.AddMovementInput` (`KismetMathLibrary.GetForwardVector` (`self.GetControlRotation`)) AxisValue))))

(event `InputAxis|Turn`
  (params (AxisValue :type "Float (single-precision)"))
  ;[1 1 1 1 15] Character control
  (`self.AddControllerYawInput` AxisValue))

(event `Ragdoll`
  ;[1 1 1 1 10] Ragdoll
  (`PrimitiveComponent.SetSimulatePhysics` (`self.Mesh`) true)
  (`CharacterMovementComponent.DisableMovement` (`self.CharacterMovement`)))

(event `InputAxis|MoveRight`
  (params (AxisValue :type "Float (single-precision)"))
  ;[1 1 1 1 15] Character control
  (`self.AddMovementInput` (`KismetMathLibrary.GetRightVector` (`self.GetControlRotation`)) AxisValue))

(event `InputAxis|LookUp`
  (params (AxisValue :type "Float (single-precision)"))
  ;[1 1 1 1 15] Character control
  (`self.AddControllerPitchInput` AxisValue))

(event `self.ReceiveAnyDamage`
  (params (Damage :type "Float (single-precision)") (DamageType :type "DamageType Object Reference") (InstigatedBy :type "Controller Object Reference") (DamageCauser :type "Actor Object Reference"))
  ;[1 1 1] When damage occurs
  (if (not (`AnimInstance.Montage_IsPlaying` (`SkeletalMeshComponent.GetAnimInstance` (`self.Mesh`)) null))
    (bind _output_get (set `self.Health` (`KismetMathLibrary.FClamp` (- (`self.Health`) Damage) 0.0 100.0)))
    (`self.PlayAnimMontage` "/Game/Animation/Hit_On_Side_Of_Body_Montage1.Hit_On_Side_Of_Body_Montage1")
    (if (== _output_get 0.0)
      (`self.Ragdoll`)
      (`/Engine/EditorBlueprintResources/StandardMacros.DoOnce` false
        (:`Completed`
          (`self.Gameover`))))))

(event `self.K2_OnMovementModeChanged`
  (params (PrevMovementMode :type "EMovementMode Enum" :default "MOVE_None") (NewMovementMode :type "EMovementMode Enum" :default "MOVE_None") (PrevCustomMode :type Byte) (NewCustomMode :type Byte))
  (bind (_returnvalue_roll _returnvalue_pitch _returnvalue_yaw) (`KismetMathLibrary.BreakRotator` (`self.K2_GetActorRotation`)))
  (bind _charactermovement (`self.CharacterMovement`))
  ;[1 1 1 1 15] Movement mode change to swimming
  (if (`|EnumEquality` NewMovementMode "MOVE_Swimming")
    (set `self.Is Swimming?` true)
    (set `CharacterMovementComponent.RotationRate` (struct :`Pitch` 600.0 :`Yaw` 600.0 :`Roll` 600.0) _charactermovement)
    (else
      (set `self.Is Swimming?` false)
      (set `CharacterMovementComponent.RotationRate` (struct :`Yaw` 540.0) _charactermovement)
      (`self.K2_SetActorRotation` (`KismetMathLibrary.MakeRotator` 0.0 0.0 _returnvalue_yaw)))))

(fn `NewFunction_0`)

(fn `UserConstructionScript`)