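; Health pickup that spins every tick and heals an overlapping BP_Character by a fixed amount, clamped to a health range.
; On pickup it hides and disables mesh collision, then reappears in place after a delay by jumping back into the BeginPlay re-enable logic, which also runs after an initial delay.
; Disconnected nodes for relocating, destroying, spawning and physics never run.
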(event `self.ReceiveTick`
  (params (DeltaSeconds :type "Float (single-precision)"))
  (bind _staticmeshcomponent (`self.StaticMeshComponent`))
  (bind (_relativerotation_roll _relativerotation_pitch _relativerotation_yaw) (`KismetMathLibrary.BreakRotator` (`SceneComponent.RelativeRotation` _staticmeshcomponent)))
  ;[1 1 1] Rotating
  (`SceneComponent.K2_SetRelativeRotation` _staticmeshcomponent (`KismetMathLibrary.MakeRotator` _relativerotation_roll _relativerotation_pitch (+ _relativerotation_yaw 2.0)) false false))

(event `self.ReceiveBeginPlay`
  (bind (_returnvalue_x _returnvalue_y _returnvalue_z) (`KismetMathLibrary.BreakVector` (`self.K2_GetActorLocation`)))
  (`KismetSystemLibrary.Delay` 3.0)
  (`PrimitiveComponent.SetCollisionEnabled` (`self.StaticMeshComponent`) "QueryAndPhysics" :!label _label)
  (set `self.Return Value Z` _returnvalue_z)
  (`self.SetActorHiddenInGame` false))

(event `self.StaticMeshComponent.OnComponentBeginOverlap`
  (params (OverlappedComponent :type "PrimitiveComponent Object Reference") (OtherActor :type "Actor Object Reference") (OtherComp :type "PrimitiveComponent Object Reference") (OtherBodyIndex :type Integer) (bFromSweep :type Boolean) (SweepResult :type "HitResult Structure (by ref)"))
  (bind _asbp_character (cast `/Game/BluePrint/BP_Character` OtherActor))
  (set `/Game/BluePrint/BP_Character.Health` (`KismetMathLibrary.FClamp` (+ (`/Game/BluePrint/BP_Character.Health` _asbp_character) 10.0) 0.0 100.0) _asbp_character)
  (`|ExecutionSequence`
    (:`then_0`
      (`KismetSystemLibrary.Delay` 3.0)
      (goto _label))
    (:`then_1`
      (`PrimitiveComponent.SetCollisionEnabled` (`self.StaticMeshComponent`) "NoCollision")
      (`self.SetActorHiddenInGame` true))))

(fn `UserConstructionScript`)