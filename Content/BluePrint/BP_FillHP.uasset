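; BP_FillHP is a health pickup that raises a BP_Character's Health on contact, then respawns elsewhere.
; Shortly after BeginPlay, its Cone enables collision and physics simulation, and the actor's current height is saved.
; When a character hits the Cone, it adds clamped health, destroys itself and spawns a replacement of its own class at a random XY within a fixed area, at the saved height.
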(event `self.ReceiveBeginPlay`
  (bind (_returnvalue_x _returnvalue_y _returnvalue_z) (`KismetMathLibrary.BreakVector` (`self.K2_GetActorLocation`)))
  (bind _cone (`self.Cone`))
  ;[1 1 1] Physics and collision setting
  (`KismetSystemLibrary.Delay` 1.0)
  (`PrimitiveComponent.SetCollisionEnabled` _cone "QueryAndPhysics")
  (`PrimitiveComponent.SetSimulatePhysics` _cone true)
  (set `self.Return Value Z` _returnvalue_z))

(event `self.Cone.OnComponentHit`
  (params (HitComponent :type "PrimitiveComponent Object Reference") (OtherActor :type "Actor Object Reference") (OtherComp :type "PrimitiveComponent Object Reference") (NormalImpulse :type "Vector Structure") (Hit :type "HitResult Structure (by ref)"))
  ;[1 1 1] Hit by character(rasing HP level) and respawn
  (bind _asbp_character (cast `/Game/BluePrint/BP_Character` OtherActor))
  (set `/Game/BluePrint/BP_Character.Health` (`KismetMathLibrary.FClamp` (+ (`/Game/BluePrint/BP_Character.Health` _asbp_character) 10.0) 0.0 100.0) _asbp_character)
  (`self.K2_DestroyActor`)
  (`|SpawnActorFromClass` "BP_FillHP_C" (`KismetMathLibrary.MakeTransform` (`KismetMathLibrary.MakeVector` (`KismetMathLibrary.RandomFloatInRange` 5000.0 6000.0) (`KismetMathLibrary.RandomFloatInRange` 645.0 2000.0) (`self.Return Value Z`)) (struct) (1.0 1.0 2.25)) "Undefined" "OverrideRootScale" null null))

(fn `UserConstructionScript`)