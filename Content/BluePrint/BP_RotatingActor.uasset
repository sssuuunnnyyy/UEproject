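; BP_RotatingActor is a moving obstacle that spins and damages the player.
; Tick adds a fixed, frame-rate-dependent rotation to MovingObstacle, and any Hit damages player 0's BP_Character, whatever was struck.
; BeginPlay finds a BP_SplineActor, and a timeline moves the actor along its spline, setting location and rotation.
; TimeToCompleteSeconds directly sets play rate, so larger values move faster; a note flags the spline movement as broken.
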(event `self.ReceiveTick`
  (params (DeltaSeconds :type "Float (single-precision)"))
  ;[1 1 1 1 15] Rotating circle
  (`SceneComponent.K2_AddRelativeRotation` (`self.MovingObstacle`) (struct :`Roll` 50.0) false false))

(event `self.ReceiveHit`
  (params (MyComp :type "PrimitiveComponent Object Reference") (Other :type "Actor Object Reference") (OtherComp :type "PrimitiveComponent Object Reference") (bSelfMoved :type Boolean) (HitLocation :type "Vector Structure") (HitNormal :type "Vector Structure") (NormalImpulse :type "Vector Structure") (Hit :type "HitResult Structure (by ref)"))
  ;[1 1 1 1 15] Apply Damage
  (bind _asbp_character (cast `/Game/BluePrint/BP_Character` (`GameplayStatics.GetPlayerCharacter` 0)))
  (`GameplayStatics.ApplyDamage` _asbp_character 10.0))

(event `self.ReceiveBeginPlay`
  ;[1 0 0] Doestn fucking work with spline actor
  (bind _returnvalue (`GameplayStatics.GetActorOfClass` "/Game/BluePrint/BP_SplineActor.BP_SplineActor_C"))
  (set `self.Spline Ref` _returnvalue)
  (`self.Move Object`))

(event `Move Object`
  (bind _spline (`/Game/BluePrint/BP_SplineActor.Spline` (`self.Spline Ref`)))
  ;[1 0 0] Doestn fucking work with spline actor
  (`TimelineComponent.SetPlayRate` (`self.Moving object`) (/ (`self.Time to complete (Seconds)`) 1.0))
  (bind (_direction _move_track) (`Timeline|Moving object`)
    (:`Update`
      (bind _returnvalue (`KismetMathLibrary.Lerp` 0.0 (`SplineComponent.GetSplineLength` (`/Game/BluePrint/BP_SplineActor.Spline` (`self.Spline Ref`))) _move_track))
      (`self.K2_SetActorTransform` (`KismetMathLibrary.MakeTransform` (`SplineComponent.GetLocationAtDistanceAlongSpline` _spline _returnvalue "World") (`SplineComponent.GetRotationAtDistanceAlongSpline` _spline _returnvalue "Local"))))))

(fn `UserConstructionScript`)