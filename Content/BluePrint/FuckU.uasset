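; FuckU is a coin pickup actor that adds its Coin value to the player character's Coins.
; Tick spins the Cylinder by a fixed roll step each frame, independent of delta time.
; Any overlap with the Cylinder plays a click sound, credits player 0's BP_Character without checking the overlapping actor, then destroys the pickup.
; Random respawn and repositioning nodes are left disconnected and never run.
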(event `self.ReceiveTick`
  (params (DeltaSeconds :type "Float (single-precision)"))
  (bind _cylinder (`self.Cylinder`))
  (bind (_relativerotation_roll _relativerotation_pitch _relativerotation_yaw) (`KismetMathLibrary.BreakRotator` (`SceneComponent.RelativeRotation` _cylinder)))
  (`SceneComponent.K2_SetRelativeRotation` _cylinder (`KismetMathLibrary.MakeRotator` (+ _relativerotation_roll 2.0) _relativerotation_pitch _relativerotation_yaw) false false))

(event `self.Cylinder.OnComponentHit`
  (params (HitComponent :type "PrimitiveComponent Object Reference") (OtherActor :type "Actor Object Reference") (OtherComp :type "PrimitiveComponent Object Reference") (NormalImpulse :type "Vector Structure") (Hit :type "HitResult Structure (by ref)")))

(event `self.Cylinder.OnComponentBeginOverlap`
  (params (OverlappedComponent :type "PrimitiveComponent Object Reference") (OtherActor :type "Actor Object Reference") (OtherComp :type "PrimitiveComponent Object Reference") (OtherBodyIndex :type Integer) (bFromSweep :type Boolean) (SweepResult :type "HitResult Structure (by ref)"))
  (`GameplayStatics.PlaySound2D` "/Engine/VREditor/Sounds/VR_click2.VR_click2" 1.0 1.0 0.0 null null)
  (bind _asbp_character (cast `/Game/BluePrint/BP_Character` (`GameplayStatics.GetPlayerCharacter` 0)))
  (set `/Game/BluePrint/BP_Character.Coins` (+ (`/Game/BluePrint/BP_Character.Coins` _asbp_character) (`self.Coin`)) _asbp_character)
  (`self.K2_DestroyActor`))

(event `self.Box.OnComponentBeginOverlap`
  (params (OverlappedComponent :type "PrimitiveComponent Object Reference") (OtherActor :type "Actor Object Reference") (OtherComp :type "PrimitiveComponent Object Reference") (OtherBodyIndex :type Integer) (bFromSweep :type Boolean) (SweepResult :type "HitResult Structure (by ref)")))

(fn `UserConstructionScript`)