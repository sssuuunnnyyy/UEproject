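; BP_Shooter is an automatic launcher actor that fires BP_Shooter_Bomb projectiles at a fixed interval.
; BeginPlay starts a looping timer that calls the Shooter 1 function by name every second.
; Each shot spawns a bomb at the Arrow component, sets its sphere's physics velocity along the arrow's forward vector, and plays an explosion particle effect at the Cylinder.
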(event `self.ReceiveBeginPlay`
  (`KismetSystemLibrary.K2_SetTimer` null "Shooter 1" 1.0 true)
  (`KismetSystemLibrary.Delay` 1.0))

(fn `Shooter 1`
  ;[1 1 1 1 10] Function for Spawning bomb to the shooter
  (bind _returnvalue (`|SpawnActorFromClass` "/Game/BluePrint/BP_Shooter_Bomb.BP_Shooter_Bomb_C" (`KismetMathLibrary.MakeTransform` (`SceneComponent.K2_GetComponentLocation` (`self.Arrow`))) "Undefined" "OverrideRootScale" null null))
  (`PrimitiveComponent.SetPhysicsLinearVelocity` (`/Game/BluePrint/BP_Shooter_Bomb.Sphere1` _returnvalue) (* (`SceneComponent.GetForwardVector` (`self.Arrow`)) 3000.0) false "None")
  (`GameplayStatics.SpawnEmitterAtLocation` "/Game/StarterContent/Particles/P_Explosion.P_Explosion" (`SceneComponent.K2_GetComponentLocation` (`self.Cylinder`))))

(fn `UserConstructionScript`)