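; Plane_Blueprint is an actor whose static mesh shuttles endlessly back and forth along its relative Y axis.
; Each Tick adds a fixed Y offset without sweep, so speed depends on frame rate rather than delta time.
; The MoveRight boolean selects the direction and flips when the mesh passes hardcoded upper or lower Y limits.
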(event `self.ReceiveTick`
  (params (DeltaSeconds :type "Float (single-precision)"))
  (bind _staticmeshcomponent (`self.StaticMeshComponent`))
  (bind (_relativelocation_x _relativelocation_y) (`KismetMathLibrary.BreakVector` (`SceneComponent.RelativeLocation` _staticmeshcomponent)))
  (bind (_relativelocation_x_2 _relativelocation_y_2) (`KismetMathLibrary.BreakVector` (`SceneComponent.RelativeLocation` _staticmeshcomponent)))
  (if (`self.Move Right`)
    (`SceneComponent.K2_AddRelativeLocation` _staticmeshcomponent (0.0 10.0 0.0) false false)
    (if (>= _relativelocation_y 1900.0)
      (set `self.Move Right` false))
    (else
      (`SceneComponent.K2_AddRelativeLocation` _staticmeshcomponent (0.0 -10.0 0.0) false false)
      (if (< _relativelocation_y_2 -1400.0)
        (set `self.Move Right` true)))))

(fn `UserConstructionScript`)