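; BP_Cones is a moving cone hazard that rises and sinks continuously and damages actors that hit it.
; Each tick, a direction flag moves the Cone component up quickly or down more slowly, flipping at upper and lower relative Z limits.
; Movement is a fixed per-frame offset without sweep, so speed depends on frame rate.
; The Hit event applies fixed damage to the other actor.
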(event `self.ReceiveTick`
  (params (DeltaSeconds :type "Float (single-precision)"))
  (bind _cone (`self.Cone`))
  (bind (_relativelocation_x _relativelocation_y _relativelocation_z) (`KismetMathLibrary.BreakVector` (`SceneComponent.RelativeLocation` _cone)))
  (bind (_relativelocation_x_2 _relativelocation_y_2 _relativelocation_z_2) (`KismetMathLibrary.BreakVector` (`SceneComponent.RelativeLocation` _cone)))
  ;[1 1 1 1 15] Moving up and down cones
  (if (`self.IsMoveUp`)
    (`SceneComponent.K2_AddRelativeLocation` _cone (0.0 0.0 15.0) false false)
    (if (>= _relativelocation_z -2.0)
      (set `self.IsMoveUp` false))
    (else
      (`SceneComponent.K2_AddRelativeLocation` _cone (0.0 0.0 -5.0) false false)
      (if (< _relativelocation_z_2 -168.0)
        (set `self.IsMoveUp` true)))))

(event `self.ReceiveHit`
  (params (MyComp :type "PrimitiveComponent Object Reference") (Other :type "Actor Object Reference") (OtherComp :type "PrimitiveComponent Object Reference") (bSelfMoved :type Boolean) (HitLocation :type "Vector Structure") (HitNormal :type "Vector Structure") (NormalImpulse :type "Vector Structure") (Hit :type "HitResult Structure (by ref)"))
  ;[1 1 1 1 15] Apply Damage
  (`GameplayStatics.ApplyDamage` Other 10.0 null self))

(fn `UserConstructionScript`)